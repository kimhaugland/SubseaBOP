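; BP_Explode2 is an actor that scatters the actors attached to a RootExplode actor, producing a rough exploded view.
; The construction script gathers the attached hierarchy into Childs, appending each child's attachments while iterating so deeper descendants are included.
; Each press of key 1 offsets every gathered actor in world space by a random amount on all three axes, with no interpolation or way back.
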(event EventBeginPlay)

(event Collision|EventActorBeginOverlap
  (params (OtherActor :type Actor%20Object%20Reference)))

(event EventTick
  (params (DeltaSeconds :type Float%20%28single-precision%29)))

(event Input|KeyboardEvents|1
  (params (Key :type Key%20Structure :default "None"))
  (bind _returnvalue (Math|Random|RandomFloatinRange -1e+02 1e+02))
  (:Pressed
    (for _array_element (Variables|Default|Getchilds)
      (Transformation|AddActorWorldOffset _array_element (Math|Vector|MakeVector _returnvalue _returnvalue _returnvalue)))))

(fn ConstructionScript
  (bind _output_get (Variables|Default|Setchilds (Actor|GetAttachedActors (Variables|Default|GetRootExplode) true)))
  (for _array_element _output_get
    (Utilities|Array|AppendArray (Variables|Default|Getchilds) (Actor|GetAttachedActors _array_element true))))