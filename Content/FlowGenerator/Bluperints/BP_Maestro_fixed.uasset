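; BP_Maestro_fixed is a sequencer that plays FlowSequence steps, launching each step's flow parts at a signed play rate, optionally auto-starting after BeginPlay.
; PlaySequence advances by calling itself after a per-step delay, optionally adding the flow's duration.
; At the end it can loop and trigger other Maestros, even on each loop pass.
; ResetMaes resets all flow parts with a Hide flag; StartMaestro is an empty stub.
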(event Custom|PlaySequence
  (params (Forward/reverse :type Float%20%28single-precision%29))
  (bind _flowsequence (Variables|Sequences|GetFlowSequence))
  (bind _returnvalue (Utilities|Array|Length _flowsequence))
  (Variables|Default|SetFlowspeed/dir Forward/reverse)
  (if (Math|Integer|InRange(Integer) (Variables|Default|GetIndex) 0 _returnvalue true false)
    (for _array_element (.flowparts (Utilities|Array|Get(acopy) (Variables|Sequences|GetFlowSequence) (Variables|Default|GetIndex))) :!label _label
      (Default|LaunchSequence _array_element (* Forward/reverse (.playrate (Utilities|Array|Get(acopy) (Variables|Sequences|GetFlowSequence) (Variables|Default|GetIndex))))))
    (if (.waitflowend (Utilities|Array|Get(acopy) (Variables|Sequences|GetFlowSequence) (Variables|Default|GetIndex)))
      ;[1 1 1] Launch the next FlowPart
      (Utilities|FlowControl|Delay (+ (/ 1.0 (.playrate (Utilities|Array|Get(acopy) (Variables|Sequences|GetFlowSequence) (Variables|Default|GetIndex)))) (.delaybeforenext (Utilities|Array|Get(acopy) (Variables|Sequences|GetFlowSequence) (Variables|Default|GetIndex)))))
      (Variables|Default|SetIndex (+ (Variables|Default|GetIndex) 1))
      (CallFunction|PlaySequence (Variables|Default|GetFlowspeed/dir))
      (else
        (Utilities|FlowControl|Delay (.delaybeforenext (Utilities|Array|Get(acopy) (Variables|Sequences|GetFlowSequence) (Variables|Default|GetIndex))))
        (Variables|Default|SetIndex (+ (Variables|Default|GetIndex) 1))
        (CallFunction|PlaySequence (Variables|Default|GetFlowspeed/dir))))
    (else
      (if (and (== (Variables|Default|GetIndex) _returnvalue) (Variables|Config|GetLoop))
        (Utilities|FlowControl|Sequence
          (:then_0
            (Variables|Default|SetIndex 0)
            (goto _label))
          (:then_1
            _)))
      (Variables|Default|SetIndex 0)
      ;[1 1 1] Play another Maestro at the end
      (if (Variables|PlayOtherMaestro|GetPlayAnotherMaestroAtEnd)
        (for _array_element_2 (Variables|PlayOtherMaestro|GetTheOtherMaestro)
          (CallFunction|PlaySequence _array_element_2 (Variables|Default|GetFlowspeed/dir)))))))

(event Custom|ResetMaes
  (params (hide :type Boolean))
  ;[1 1 1] Reset : Usefull when looping
  (for _array_element (Variables|Sequences|GetFlowSequence)
    (for _array_element_2 (.flowparts _array_element)
      (Default|Reset _array_element_2 hide))))

(event EventBeginPlay
  (Variables|Default|SetIndex 0)
  (if (Variables|Config|GetAutoPlay)
    ;[0 0 0 1 12] Wait a little bit until all the flow parts are built in the level
    (Utilities|FlowControl|Delay 1.0)
    (CallFunction|PlaySequence 1.0)))

(fn ConstructionScript)

(fn StartMaestro
  (params (NameOfMaestro :type String) (FlowDirection :type Float%20%28single-precision%29)))