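; Flow segment actor that builds spline meshes along a spline and displays directional flow through material parameters.
; The construction script creates one mesh per spline segment, optionally feeds world positions to listed static meshes' materials and hides the particle trail when disabled.
; Meshes start hidden; LaunchSequence shows them red for positive rates or blue for negative, passing the rate as Speed.
; Zero rate or Reset hides them again; PlayPause is empty.
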(event Custom|LaunchSequence
  (params (PlayRate :type Float%20%28single-precision%29))
  (Math|Float|CompareFloat PlayRate 0.0
    (:>
      (for _array_element (Variables|Default|GetSplineMesh)
        (Rendering|Material|SetVectorParameterValueonMaterials _array_element "normal" "1.000000, 0, 0")
        (Rendering|Material|SetMaterial _array_element 0 (Variables|Config|GetMat))
        (Rendering|Material|SetVectorParameterValueonMaterials _array_element "EmiColor" (Math|Conversions|ToVector(LinearColor) (Math|Conversions|ToLinearColor(Color) (Class|KismetMathLibrary|LinearColortoRGBE "(R=1.000000,G=0.000000,B=0.054744,A=1.000000)"))))
        (Rendering|Material|SetScalarParameterValueonMaterials _array_element "Speed" PlayRate)
        (Rendering|SetVisibility _array_element true false)))
    (:==
      (for _array_element_2 (Variables|Default|GetSplineMesh)
        (Rendering|Material|SetVectorParameterValueonMaterials _array_element_2 "normal" "0, 0, 0")
        (Rendering|SetVisibility _array_element_2 false false)))
    (:<
      (for _array_element_3 (Variables|Default|GetSplineMesh)
        (Rendering|Material|SetVectorParameterValueonMaterials _array_element_3 "normal" "1.000000, 0, 0")
        (Rendering|Material|SetVectorParameterValueonMaterials _array_element_3 "EmiColor" (Math|Conversions|ToVector(LinearColor) (Math|Conversions|ToLinearColor(Color) (Class|KismetMathLibrary|LinearColortoRGBE "(R=0.000000,G=0.043967,B=1.000000,A=1.000000)"))))
        (Rendering|Material|SetScalarParameterValueonMaterials _array_element_3 "Speed" PlayRate)
        (Rendering|SetVisibility _array_element_3 true false)))))

(event Custom|PlayPause
  (params (PLayRate :type Float%20%28single-precision%29)))

(event Custom|Reset
  (params (hide :type Boolean))
  (for _array_element (Variables|Default|GetSplineMesh)
    (Rendering|Material|SetVectorParameterValueonMaterials _array_element "normal" "0, 0, 0")
    (Rendering|SetVisibility _array_element false false)))

(event EventBeginPlay
  (for _array_element (Variables|Default|GetSplineMesh)
    (Rendering|Material|SetVectorParameterValueonMaterials _array_element "normal" "0, 0, 0")
    (Rendering|SetVisibility _array_element false false)))

(fn ConstructionScript
  (Utilities|IsValid (Variables|Config|GetStaticMesh)
    (:Is%20Valid
      (CallFunction|BuildSpline))
    (:Is%20Not%20Valid
      _))
  (if (Variables|Config|GetSpawnParticle)
    _
    (else
      (Rendering|SetVisibility (Variables|Default|GetP_Trail_Trace) false false)))
  (if (Variables|FlowStaticMeshes|GetFlowStaticMesh)
    (for _array_element (Variables|FlowStaticMeshes|GetStaticMeshes)
      (Rendering|Material|SetVectorParameterValueonMaterials (Variables|/Script/Engine.StaticMeshActor|GetStaticMeshComponent _array_element) "normal" "1.000000,0.000000,0.000000")
      (Rendering|Material|SetVectorParameterValueonMaterials (Variables|/Script/Engine.StaticMeshActor|GetStaticMeshComponent _array_element) "pos" (Transformation|GetWorldLocation (Variables|/Script/Engine.StaticMeshActor|GetStaticMeshComponent _array_element))))))

(fn BuildSpline
  (bind _spline (Variables|Default|GetSpline))
  (bind _splinescale (Variables|Config|GetSplineScale))
  (Utilities|Array|Clear (Variables|Default|GetSplineMesh))
  (for _index (range 0 (- (Spline|GetNumberOfSplinePoints (Variables|Default|GetSpline)) 2))
    (bind _returnvalue (AddComponent|AddSplineMeshComponent false))
    (Utilities|Array|AddUnique (Variables|Default|GetSplineMesh) _returnvalue)
    (Components|StaticMesh|SetStaticMesh _returnvalue (Variables|Config|GetStaticMesh))
    (Rendering|Material|SetMaterial _returnvalue 0 (Variables|Config|GetMat))
    (SplineMesh|SetForwardAxis _returnvalue (Variables|Config|GetForwardAxis) true)
    (Transformation|AttachComponentToComponent _returnvalue (Variables|Default|GetSpline) "None" "KeepRelative" "KeepRelative" "KeepRelative" true)
    (SplineMesh|SetStartandEnd _returnvalue (Spline|GetLocationatSplinePoint _spline _index "Local") (Spline|GetTangentatSplinePoint _spline _index "Local") (Spline|GetLocationatSplinePoint _spline (+ _index 1) "Local") (Spline|GetTangentatSplinePoint _spline (+ _index 1) "Local") true :!class /Script/Engine.SplineMeshComponent)
    (SplineMesh|SetEndScale _returnvalue _splinescale true :!class /Script/Engine.SplineMeshComponent)
    (SplineMesh|SetStartScale _returnvalue _splinescale true :!class /Script/Engine.SplineMeshComponent)
    (Rendering|SetCastShadow _returnvalue (Variables|Config|GetCastShadow))))

(fn ResetAllMat
  (if (not (Variables|FlowStaticMeshes|GetFlowStaticMesh))
    (for _array_element (Variables|Default|GetSplineMesh)
      (Rendering|Material|SetVectorParameterValueonMaterials _array_element "pos" "0, 0, 0")
      (Rendering|Material|SetVectorParameterValueonMaterials _array_element "normal" "0, 0, 0"))))